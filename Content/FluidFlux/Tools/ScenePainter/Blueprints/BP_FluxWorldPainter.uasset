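; World painter actor that renders scene brushes into a PaintMap render target covering an axis-aligned area sized by resolution and pixel size.
; Construction recreates the target, configures the brush material, renders through FluxScenePainterComponent and notifies all BPI_FluxSurface actors; BeginPlay renders again.
; The repaint event has every BP_FluxWorldBrush draw itself via the painter component.
; ApplyMaterialParameters passes the map and area transform to materials, including the debug preview's.
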(event `self.ReceiveBeginPlay`
  (`self.RenderScenePainter`))

(event `self.RenderScenePainter`
  (`KismetRenderingLibrary.ClearRenderTarget2D` (`self.PaintMap`))
  (`/Game/FluidFlux/Tools/ScenePainter/Blueprints/BP_FluxWorldPainterComponent.RenderScene` (`self.FluxScenePainterComponent`) (`self.PaintMap`)))

(event `self.ApplyMaterialParameters`
  (params (Materials :type "Array of MaterialInstanceDynamic Object Reference (by ref)"))
  (`/Game/FluidFlux/Tools/ScenePainter/Blueprints/BP_FluxWorldPainterComponent.SetPainterParameters` (`self.FluxScenePainterComponent`) Materials (`KismetMathLibrary.MakeTransform` (`self.K2_GetActorLocation`) (struct) (`SceneComponent.K2_GetComponentScale` (`self.Box`))) (`self.PaintMap`)))

(event `self.OnRepaintBrushes`
  (`self.Repaint`))

(fn `InitializeDebug`
  (`/Engine/EditorBlueprintResources/StandardMacros.IsValid` (`self.Preview`)
    (:`Is Valid`
      (bind _returnvalue (`KismetMaterialLibrary.CreateDynamicMaterialInstance` "/Game/FluidFlux/Tools/ScenePainter/Materials/M_ScenePainterPreview.M_ScenePainterPreview"))
      (set `self.DebugPaintMap` _returnvalue)
      (`PrimitiveComponent.SetMaterial` (`self.Preview`) 0 (`self.DebugPaintMap`))
      (bind _returnvalue_2 (`KismetSystemLibrary.LoadAsset_Blocking` (`self.DebugMesh`)))
      (bind _asstatic_mesh (cast `StaticMesh` _returnvalue_2))
      (`StaticMeshComponent.SetStaticMesh` (`self.Preview`) _asstatic_mesh)
      (`self.ApplyMaterialParameters` (`|MakeArray` (`self.DebugPaintMap`))))))

(fn `Repaint`
  (locals (Actors :type "Array of /Game/FluidFlux/Tools/ScenePainter/Blueprints/BP_FluxWorldBrush Object Reference"))
  (bind _outactors (`GameplayStatics.GetAllActorsOfClass` "/Game/FluidFlux/Tools/ScenePainter/Blueprints/BP_FluxWorldBrush.BP_FluxWorldBrush_C"))
  (set `local.Actors` _outactors)
  (for _array_element (`local.Actors`)
    (`/Game/FluidFlux/Tools/ScenePainter/Blueprints/BP_FluxWorldBrush.Draw` _array_element (`self.BrushMaterialIntance`) (`self.FluxScenePainterComponent`))))

(fn `UserConstructionScript`
  (bind (_arearesolution_x _arearesolution_y) (break `IntPoint` (`self.AreaResolution`)))
  (bind (_returnvalue_x _returnvalue_y) (`KismetMathLibrary.BreakVector` (`KismetMathLibrary.Conv_Vector2DToVector` (* (`KismetMathLibrary.Conv_IntPointToVector2D` (`self.AreaResolution`)) (`self.AreaPixelSize`)) (`self.AreaPixelSize`))))
  (`self.K2_SetActorRotation` (struct))
  (`|ExecutionSequence`
    (:`then_0`
      (bind _newtexture (`/Game/FluidFlux/Editor/Blueprints/BPL_FluidFlux.RecreateRenderTarget` (`self.PaintMap`) _arearesolution_x _arearesolution_y "RTF_R8" (struct :`A` 1.0)))
      (bind _output_get (set `self.PaintMap` _newtexture))
      (`/Game/FluidFlux/Editor/Blueprints/BPL_FluidFlux.SetRenderTargetConfig` _output_get))
    (:`then_1`
      (`SceneComponent.SetWorldScale3D` (`self.Box`) (`KismetMathLibrary.MakeVector` _returnvalue_x _returnvalue_y 1.0))
      (bind _returnvalue (`KismetMaterialLibrary.CreateDynamicMaterialInstance` "/Game/FluidFlux/Tools/ScenePainter/Materials/MI_SceneBrush.MI_SceneBrush"))
      (bind _output_get_2 (set `self.BrushMaterialIntance` _returnvalue))
      (`/Game/FluidFlux/Tools/ScenePainter/Blueprints/BP_FluxWorldPainterComponent.SetBrushParameters` (`self.FluxScenePainterComponent`) _output_get_2 (`KismetMathLibrary.MakeTransform` (`self.K2_GetActorLocation`) (struct) (`SceneComponent.K2_GetComponentScale` (`self.Box`))) (`self.AreaResolution`)))
    (:`then_2`
      (`self.RenderScenePainter`))
    (:`then_3`
      (bind _preview (`self.Preview`)
        (:`then`
          (`SceneComponent.SetVisibility` _preview (`self.DrawDebug`) false))
        (:`else`)))
    (:`then_4`
      (bind _outactors (`GameplayStatics.GetAllActorsWithInterface` "/Game/FluidFlux/Surface/Blueprints/BPI_FluxSurface.BPI_FluxSurface_C"))
      (for _array_element _outactors
        (message `/Game/FluidFlux/Surface/Blueprints/BPI_FluxSurface.ApplyPainter` _array_element)))
    (:`then_5`
      (`self.InitializeDebug`))))