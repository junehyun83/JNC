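; Fluid Flux tool actor that bakes hand-shaped spline curves into an animated wave profile data asset and passes it to a wave actor.
; It samples the curves across wave width and time, drawing range-remapped offsets and foam into a forward render target.
; A scene capture renders inverse maps at two scales, which a material combines into one.
; The rebuild runs on construction and BeginPlay, also updating preview materials.
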(event `self.ReceiveBeginPlay`
  (`self.Initialize`))

(fn `BuildProfile`
  (`|ExecutionSequence`
    (:`then_0`
      (`self.Generate Wave Profile`)
      (`self.CreateProfile`)
      (`|ExecutionSequence`
        (:`then_0`
          (bind _returnvalue (`PrimitiveComponent.CreateDynamicMaterialInstance` (`self.PreviewForward`) 0 "/Game/FluidFlux/Tools/WaveProfile/Materials/M_WaveProfileForward.M_WaveProfileForward" "None"))
          (set `self.WaveForwardPreviewInstance` _returnvalue))
        (:`then_1`
          (bind _returnvalue_2 (`PrimitiveComponent.CreateDynamicMaterialInstance` (`self.PreviewInverse`) 0 "/Game/FluidFlux/Tools/WaveProfile/Materials/M_WaveProfileInverse.M_WaveProfileInverse" "None"))
          (set `self.WaveInversePreviewInstance` _returnvalue_2))
        (:`then_2`
          (bind _returnvalue_3 (`PrimitiveComponent.CreateDynamicMaterialInstance` (`self.Animation`) 0 null "None"))
          (set `self.WaveAnimation` _returnvalue_3))
        (:`then_3`
          (bind _returnvalue_4 (`PrimitiveComponent.CreateDynamicMaterialInstance` (`self.RenderInverse`) 0 null "None"))
          (set `self.WaveInverseRender` _returnvalue_4))
        (:`then_4`
          (`/Game/FluidFlux/Tools/WaveProfile/Blueprints/PDA_FluxWaveProfile.ApplyWaveProfileMaterialData` (`self.WaveProfile`) (`|MakeArray` (`self.WaveInverseRender`) (`self.WaveAnimation`) (`self.WaveForwardPreviewInstance`) (`self.WaveInversePreviewInstance`))))))
    (:`then_1`
      (`self.CaptureInverseMap` (`self.WaveProfilesInverseMap_05`) 0.5)
      (`self.CaptureInverseMap` (`self.WaveProfilesInverseMap_10`))
      (bind _returnvalue_5 (`KismetMaterialLibrary.CreateDynamicMaterialInstance` "/Game/FluidFlux/Tools/WaveProfile/Materials/M_CombineInversemaps.M_CombineInversemaps"))
      (`MaterialInstanceDynamic.SetTextureParameterValue` _returnvalue_5 "InvMap_05" (`self.WaveProfilesInverseMap_05`))
      (`MaterialInstanceDynamic.SetTextureParameterValue` _returnvalue_5 "InvMap_10" (`self.WaveProfilesInverseMap_10`))
      (`KismetRenderingLibrary.DrawMaterialToRenderTarget` (`self.WaveProfilesInverseMap`) _returnvalue_5))
    (:`then_2`
      (bind _waveactor (`self.WaveActor`)
        (:`then`
          (message `/Game/FluidFlux/Waves/Blueprints/BPI_FluxWaveRenderer.SetWaveProfile` _waveactor (`self.WaveProfile`)))
        (:`else`)))))

(fn `CaptureInverseMap`
  (params (`Texture Target` :type "TextureRenderTarget2D Object Reference") (Scale :type "Float (double-precision)" :default 1.0))
  (`MaterialInstanceDynamic.SetScalarParameterValue` (`self.WaveInverseRender`) "Scale" Scale)
  (set `SceneCaptureComponent2D.TextureTarget` (`local.Texture Target`) (`self.SceneCapture`))
  (set `SceneCaptureComponent.ShowOnlyActors` (`|MakeArray` self :!type "Actor Object Reference") (`self.SceneCapture`))
  (`SceneCaptureComponent2D.CaptureScene` (`self.SceneCapture`)))

(fn `ClearRemap`
  (set `self.RemapX` (-0.1 0.1))
  (set `self.RemapY` (0.0 0.05)))

(fn `CreateProfile`
  (`|ExecutionSequence`
    (:`then_0`
      (`/Engine/EditorBlueprintResources/StandardMacros.IsValid` (`self.WaveProfile`)
        (:`Is Not Valid`
          (bind _returnvalue (`|GenericCreateObject` self "/Game/FluidFlux/Tools/WaveProfile/Blueprints/PDA_FluxWaveProfile.PDA_FluxWaveProfile_C"))
          (set `self.WaveProfile` _returnvalue))))
    (:`then_1`
      (`/Game/FluidFlux/Tools/WaveProfile/Blueprints/PDA_FluxWaveProfile.SetWaveProfileData` (`self.WaveProfile`) (`self.WaveProfilesForwardMap`) (`self.WaveProfilesInverseMap`) (`self.WaveProfileDecode`) (`KismetArrayLibrary.Array_Length` (`self.Curves`)) (`self.WaveWidth`) (`self.WaveHeight`)))))

(fn `Generate Wave Profile`
  (locals (StartPoint :type "Vector Structure" :default (0.0 0.0 0.0)) (CurrentSpline :type "SplineComponent Object Reference") (Y :type "Float (double-precision)" :default 0.0) (X :type "Float (double-precision)" :default 0.0) (Canvas :type "Canvas Object Reference") (SplineWidth :type "Float (double-precision)" :default 0.0) (PiointMaterial :type "MaterialInstanceDynamic Object Reference") (RendeContext :type "DrawToRenderTargetContext Structure") (Sample :type "LinearColor Structure"))
  (bind (_remapy_x _remapy_y) (`KismetMathLibrary.BreakVector2D` (`self.RemapY`)))
  (bind (_remapx_x _remapx_y) (`KismetMathLibrary.BreakVector2D` (`self.RemapX`)))
  (bind (_remapy_x_2 _remapy_y_2) (`KismetMathLibrary.BreakVector2D` (`self.RemapY`)))
  (bind (_remapx_x_2 _remapx_y_2) (`KismetMathLibrary.BreakVector2D` (`self.RemapX`)))
  (bind (_sample_r _sample_g) (break `LinearColor` (`local.Sample`)))
  (bind (_sample_r_2 _sample_g_2) (break `LinearColor` (`local.Sample`)))
  (bind _sample_r_3 (break `LinearColor` (`local.Sample`)))
  (bind (_remapy_x_3 _remapy_y_3) (`KismetMathLibrary.BreakVector2D` (`self.RemapY`)))
  (bind (_sample_r_4 _sample_g_3 _sample_b _sample_a) (break `LinearColor` (`local.Sample`)))
  (bind (_remapx_x_3 _remapx_y_3) (`KismetMathLibrary.BreakVector2D` (`self.RemapX`)))
  (bind _sample_r_5 (break `LinearColor` (`local.Sample`)))
  (bind (_remapy_x_4 _remapy_y_4) (`KismetMathLibrary.BreakVector2D` (`self.RemapY`)))
  (bind _returnvalue (- _remapy_y_2 _remapy_x_2))
  (bind _returnvalue_2 (- _remapx_y _remapx_x))
  (bind _returnvalue_3 (/ (+ (`local.X`) 0.5) (`KismetMathLibrary.Conv_IntToDouble` (- (`self.CurveSamples(X)`) 0))))
  (bind _returnvalue_4 (* (/ (+ (`local.Y`) 0.0) (- (`KismetMathLibrary.Conv_IntToDouble` (`self.TimeSamples(Y)`)) 1.0)) (/ (`KismetMathLibrary.Conv_IntToDouble` (`self.TimeSamples(Y)`)) (`KismetMathLibrary.Conv_IntToDouble` (+ (`self.TimeSamples(Y)`) 1)))))
  (bind _returnvalue_5 (`KismetMathLibrary.MakeColor` (- (/ (.x (`SplineComponent.GetLocationAtTime` (`self.Soft`) _returnvalue_4 "Local" false)) (`local.SplineWidth`)) _returnvalue_3) (/ (.z (`SplineComponent.GetLocationAtTime` (`self.Soft`) _returnvalue_4 "Local" false)) (`local.SplineWidth`)) (* (* (`KismetMathLibrary.FClamp` (- 1.0 (/ (`KismetMathLibrary.Abs` (- _returnvalue_3 (.x (`SplineComponent.GetLocationAtTime` (`self.Foam`) _returnvalue_4 "Local" false)))) (`KismetMathLibrary.FMax` (.z (`SplineComponent.GetLocationAtTime` (`self.Foam`) _returnvalue_4 "Local" false)) 1e-06)))) 1.0) (.y (`SplineComponent.GetLocationAtTime` (`self.Foam`) _returnvalue_4 "Local" false)))))
  (set `self.WaveHeight` 0)
  (`|ExecutionSequence`
    (:`then_0`
      (bind _returnvalue_6 (`KismetMaterialLibrary.CreateDynamicMaterialInstance` (`self.DrawPointMaterial`)))
      (set `local.PiointMaterial` _returnvalue_6))
    (:`then_1`
      (bind (_canvas _size _context) (`KismetRenderingLibrary.BeginDrawCanvasToRenderTarget` (`self.WaveProfilesForwardMap`)))
      (set `local.Canvas` _canvas)
      (set `local.RendeContext` _context)
      (`local.Canvas`
        (:`then`
          (set `local.SplineWidth` (`KismetMathLibrary.Conv_IntToDouble` (`self.WaveWidth`)))
          (for _index (range (`self.CurveSamples(X)`))
            (set `local.X` (`KismetMathLibrary.Conv_IntToDouble` _index))
            (`self.LoadSpline` _returnvalue_3)
            (for _index_2 (range (`self.TimeSamples(Y)`))
              (set `local.Y` (`KismetMathLibrary.Conv_IntToDouble` _index_2))
              (set `local.Sample` (`KismetMathLibrary.LinearColorLerp` _returnvalue_5 (* _returnvalue_5 (`KismetMathLibrary.MakeColor` 1.0 0.5)) (- 1.0 (`KismetMathLibrary.FClamp` (* 4 (- 1.0 (`KismetMathLibrary.Abs` (- (* (/ (`KismetMathLibrary.Conv_IntToDouble` _index) (`KismetMathLibrary.Conv_IntToDouble` (- (`self.CurveSamples(X)`) 1))) 2.0) 1.0))))))))
              (`|ExecutionSequence`
                (:`then_0`
                  (`MaterialInstanceDynamic.SetVectorParameterValue` (`local.PiointMaterial`) "Color" (make `LinearColor` (`KismetMathLibrary.MapRangeClamped` _sample_r_5 _remapx_x_3 _remapx_y_3 0.0 1.0) (`KismetMathLibrary.MapRangeClamped` _sample_g_2 _remapy_x_3 _remapy_y_3 0.0 1.0) _sample_b _sample_a))
                  (`Canvas.K2_DrawMaterial` (`local.Canvas`) (`local.PiointMaterial`) (`KismetMathLibrary.MakeVector2D` (+ (`local.X`) 0.5) (+ (`local.Y`) 0.5)) (1.0 1.0) (0.0 0.0) (1.0 1.0) 0.0 (0.5 0.5)))
                (:`then_1`
                  (set `self.RemapX` (`KismetMathLibrary.MakeVector2D` (`KismetMathLibrary.FMin` _sample_r_3 _remapx_x_2) (`KismetMathLibrary.FMax` _sample_r_3 _remapx_y_2)))
                  (set `self.RemapY` (`KismetMathLibrary.MakeVector2D` (`KismetMathLibrary.FMax` (`KismetMathLibrary.FMin` _sample_g _remapy_x_4)) (`KismetMathLibrary.FMax` _sample_g _remapy_y_4)))
                  (set `self.WaveHeight` (`KismetMathLibrary.FTrunc` (* _remapy_y (`local.SplineWidth`)))))))))
        (:`else`)))
    (:`then_2`
      (`KismetRenderingLibrary.EndDrawCanvasToRenderTarget` (`local.RendeContext`)))
    (:`then_3`
      (set `self.WaveProfileDecode` (`KismetMathLibrary.MakeColor` (/ _remapx_x _returnvalue_2) (/ _remapy_x_2 _returnvalue) _returnvalue_2 _returnvalue)))))

(fn `GetProfileSplines`
  (returns (Components :type "Array of SplineComponent Object Reference"))
  (bind _spline0last2 (`self.Spline0Last2`))
  (return (`|MakeArray` (`self.Spline019`) (`self.Spline018`) (`self.Spline014`) (`self.Spline00`) (`self.Spline01`) (`self.Spline02`) (`self.Spline03`) (`self.Spline04`) (`self.Spline05`) (`self.Spline06`) (`self.Spline07`) (`self.Spline08`) (`self.Spline09`) (`self.Spline010`) (`self.Spline012`) (`self.Spline013`) (`self.Spline011`) (`self.Spline0Last1`) _spline0last2 _spline0last2 (`self.Spline0Last`))))

(fn `Initialize`
  (`|ExecutionSequence`
    (:`then_0`
      (`self.InitRenderTargets`))
    (:`then_1`
      (bind _components (message `/Game/FluidFlux/Tools/WaveProfile/Blueprints/BPI_WaveProfileDataSource.GetProfileSplines` (select `bool` (`KismetSystemLibrary.IsValid` (`self.Source`)) :`false` self :`true` (`self.Source`) :!type "Actor Object Reference")))
      (bind _output_get (set `self.Curves` _components))
      (`KismetArrayLibrary.Array_RemoveItem` _output_get)
      (for (_array_element _array_index) (`self.Curves`)
        (`SceneComponent.K2_SetRelativeLocation` _array_element (`KismetMathLibrary.MakeVector` 0.0 (* (`KismetMathLibrary.Conv_IntToDouble` _array_index) 100.0)) false false)))
    (:`then_2`
      (`SceneComponent.SetRelativeScale3D` (`self.PreviewForward`) (`KismetMathLibrary.MakeVector` 10.0 (- (`KismetMathLibrary.Conv_IntToDouble` (`KismetArrayLibrary.Array_Length` (`self.Curves`))) 0.0) 1.0))
      (`SceneComponent.SetRelativeScale3D` (`self.PreviewInverse`) (`KismetMathLibrary.MakeVector` 10.0 (- (`KismetMathLibrary.Conv_IntToDouble` (`KismetArrayLibrary.Array_Length` (`self.Curves`))) 0.0) 1.0))
      (`SceneComponent.K2_SetRelativeLocation` (`self.PreviewForward`) (`KismetMathLibrary.MakeVector` 500.0 (+ (`KismetMathLibrary.Conv_IntToDouble` (* (`KismetArrayLibrary.Array_Length` (`self.Curves`)) 50)) (* -50 (/ (`KismetMathLibrary.Conv_IntToDouble` (`KismetArrayLibrary.Array_Length` (`self.Curves`))) (`KismetMathLibrary.Conv_IntToDouble` (`self.TimeSamples(Y)`))))) -0.1) false false)
      (`SceneComponent.K2_SetRelativeLocation` (`self.PreviewInverse`) (`KismetMathLibrary.MakeVector` 500.0 (+ (`KismetMathLibrary.Conv_IntToDouble` (* (`KismetArrayLibrary.Array_Length` (`self.Curves`)) 50)) (* -50 (/ (`KismetMathLibrary.Conv_IntToDouble` (`KismetArrayLibrary.Array_Length` (`self.Curves`))) (`KismetMathLibrary.Conv_IntToDouble` (`self.TimeSamples(Y)`))))) -0.1) false false))
    (:`then_3`
      (`SceneComponent.SetRelativeScale3D` (`self.RenderInverse`) (* (`KismetMathLibrary.MakeVector` 1.0 (/ (`KismetMathLibrary.Conv_IntToDouble` (`self.TimeSamples(Y)`)) (`KismetMathLibrary.Conv_IntToDouble` (`self.CurveSamples(X)`))) 1.0) 12.0)))
    (:`then_4`
      (`self.BuildProfile`))))

(fn `InitRenderTargets`
  (`|ExecutionSequence`
    (:`then_0`
      (bind _newtexture (`/Game/FluidFlux/Editor/Blueprints/BPL_FluidFlux.RecreateRenderTarget` (`self.WaveProfilesForwardMap`) (`self.CurveSamples(X)`) (`self.TimeSamples(Y)`) (`self.Format`) (struct) 0 true))
      (bind _output_get (set `self.WaveProfilesForwardMap` _newtexture))
      (`/Game/FluidFlux/Editor/Blueprints/BPL_FluidFlux.SetRenderTargetConfig` _output_get "TF_Bilinear" false "TA_Wrap")
      (set `Texture.MipGenSettings` "TMGS_Sharpen1" _output_get))
    (:`then_1`
      (bind _newtexture_2 (`/Game/FluidFlux/Editor/Blueprints/BPL_FluidFlux.RecreateRenderTarget` (`self.WaveProfilesInverseMap`) (`self.CurveSamples(X)`) (`self.TimeSamples(Y)`) (`self.Format`) (struct :`R` 1.0 :`G` 0.587348 :`B` 0.932053 :`A` 1.0) 0 true))
      (bind _output_get_2 (set `self.WaveProfilesInverseMap` _newtexture_2))
      (`/Game/FluidFlux/Editor/Blueprints/BPL_FluidFlux.SetRenderTargetConfig` _output_get_2 "TF_Bilinear" false "TA_Wrap")
      (set `Texture.MipGenSettings` "TMGS_Sharpen1" _output_get_2)
      (`KismetRenderingLibrary.ClearRenderTarget2D` (`self.WaveProfilesInverseMap`) (struct :`R` 0.579167 :`G` 0.057915 :`B` 0.198024)))
    (:`then_2`
      (bind _newtexture_3 (`/Game/FluidFlux/Editor/Blueprints/BPL_FluidFlux.RecreateRenderTarget` (`self.WaveProfilesInverseMap_05`) (`self.CurveSamples(X)`) (`self.TimeSamples(Y)`) (`self.Format`) (struct :`R` 1.0 :`G` 0.587348 :`B` 0.932053 :`A` 1.0) 0 true))
      (bind _output_get_3 (set `self.WaveProfilesInverseMap_05` _newtexture_3))
      (`/Game/FluidFlux/Editor/Blueprints/BPL_FluidFlux.SetRenderTargetConfig` _output_get_3 "TF_Bilinear" false "TA_Wrap"))
    (:`then_3`
      (bind _newtexture_4 (`/Game/FluidFlux/Editor/Blueprints/BPL_FluidFlux.RecreateRenderTarget` (`self.WaveProfilesInverseMap_10`) (`self.CurveSamples(X)`) (`self.TimeSamples(Y)`) (`self.Format`) (struct :`R` 1.0 :`G` 0.587348 :`B` 0.932053 :`A` 1.0) 0 true))
      (bind _output_get_4 (set `self.WaveProfilesInverseMap_10` _newtexture_4))
      (`/Game/FluidFlux/Editor/Blueprints/BPL_FluidFlux.SetRenderTargetConfig` _output_get_4 "TF_Bilinear" false "TA_Wrap"))))

(fn `LoadSpline`
  (params (SplineTime :type "Float (double-precision)"))
  (locals (X :type "Float (double-precision)") (CurrentSpline :type "SplineComponent Object Reference") (Average :type "Vector Structure" :default (0.0 0.0 0.0)))
  (bind _returnvalue (`KismetArrayLibrary.Array_Length` (`self.Curves`)))
  (`|ExecutionSequence`
    (:`then_0`
      (`SplineComponent.ClearSplinePoints` (`self.Soft`) true)
      (for _index (range (+ _returnvalue 1))
        (set `local.CurrentSpline` (`|GetArrayItem` (`self.Curves`) (`KismetMathLibrary.Min` _index (- _returnvalue 1))))
        (`SplineComponent.AddSplinePoint` (`self.Soft`) (+ (`SplineComponent.GetLocationAtTime` (`local.CurrentSpline`) (`local.SplineTime`) "Local" false) (`KismetMathLibrary.MakeVector` 0.0 (`KismetMathLibrary.Conv_IntToDouble` (* _index 100)))) "Local" false))
      ;[1 1 1] Correct start and end
      (`SplineComponent.UpdateSpline` (`self.Soft`))
      (set `local.Average` (`KismetMathLibrary.VLerp` (`SplineComponent.GetTangentAtSplinePoint` (`self.Soft`) 0 "Local") (`SplineComponent.GetTangentAtSplinePoint` (`self.Soft`) (- (`SplineComponent.GetNumberOfSplinePoints` (`self.Soft`)) 1) "Local") 0.5))
      (`SplineComponent.SetTangentAtSplinePoint` (`self.Soft`) 0 (`local.Average`) "Local" true)
      (`SplineComponent.SetTangentAtSplinePoint` (`self.Soft`) (`KismetArrayLibrary.Array_Length` (`self.Curves`)) (`local.Average`) "Local" true))
    (:`then_1`
      (`SplineComponent.ClearSplinePoints` (`self.Foam`) true)
      (for _array_element (`self.FoamPoints`)
        (`SplineComponent.AddSplinePoint` (`self.Foam`) (`KismetMathLibrary.MakeVector` (break `/Game/FluidFlux/Tools/WaveProfile/Blueprints/BS_FluxWaveProfilePoint` _array_element) (* (`.Intensity_4_B3288C7A42851B36490DC0BAFA2047B9` (break `/Game/FluidFlux/Tools/WaveProfile/Blueprints/BS_FluxWaveProfilePoint` _array_element)) (`self.FoamIntensity`)) (`.Radius_7_D0A1A43C4FECF3ECFE0279ADCBE52DA5` (break `/Game/FluidFlux/Tools/WaveProfile/Blueprints/BS_FluxWaveProfilePoint` _array_element))) "Local" false))
      (`SplineComponent.UpdateSpline` (`self.Foam`)))))

(fn `UserConstructionScript`
  (`self.Initialize`)
  (for _array_element (`self.K2_GetComponentsByClass` self "/Script/Engine.SplineComponent")
    (set `SplineComponent.bInputSplinePointsToConstructionScript` true _array_element)))